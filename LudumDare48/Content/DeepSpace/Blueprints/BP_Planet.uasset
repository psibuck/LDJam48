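; BP_Planet is a planet actor that acts as a refuelling point for the player ship.
; Entering the PlanetSupplyCollider starts refuelling on an overlapping PlayerShip, and leaving it stops refuelling.
; The construction script gives the planet sphere a random material from PlanetMaterialList, so the look is re-rolled whenever construction runs.
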(event OnComponentBeginOverlap(PlanetSupplyCollider)
  (params (OverlappedComponent :type Primitive%20Component%20Object%20Reference) (OtherActor :type Actor%20Object%20Reference) (OtherComp :type Primitive%20Component%20Object%20Reference) (OtherBodyIndex :type Integer) (bFromSweep :type Boolean) (SweepResult :type Hit%20Result%20Structure%20%28by%20ref%29))
  (bind _asplayer_ship (Utilities|Casting|CastToPlayerShip OtherActor))
  (Class|PlayerShip|StartRefuelling _asplayer_ship))

(event OnComponentEndOverlap(PlanetSupplyCollider)
  (params (OverlappedComponent :type Primitive%20Component%20Object%20Reference) (OtherActor :type Actor%20Object%20Reference) (OtherComp :type Primitive%20Component%20Object%20Reference) (OtherBodyIndex :type Integer))
  (bind _asplayer_ship (Utilities|Casting|CastToPlayerShip OtherActor))
  (Class|PlayerShip|StopRefuelling _asplayer_ship))

(event EventBeginPlay)

(event Collision|EventActorBeginOverlap
  (params (OtherActor :type Actor%20Object%20Reference)))

(event EventTick
  (params (DeltaSeconds :type Float%20%28single-precision%29)))

(fn ConstructionScript
  (Rendering|Material|SetMaterial (Variables|Default|GetPlanetSphere) 0 (Utilities|Array|Get(acopy) (Variables|Default|GetplanetMaterialList) (Math|Random|RandomInteger (Utilities|Array|Length (Variables|Default|GetplanetMaterialList))))))