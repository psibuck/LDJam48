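; BP_Asteroid is a space asteroid that breaks apart when it overlaps the player ship, another asteroid or a planet.
; A player ship hit first calls the ship's collision handler; all three cases then damage the destructible component along the asteroid's velocity and destroy the actor after a short delay.
; The construction script picks a material from a list separately for the sphere and destructible components, so the two can differ.
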(event Collision|EventActorBeginOverlap
  (params (OtherActor :type Actor%20Object%20Reference))
  (bind _asbp_player_ship (Utilities|Casting|CastToBP_PlayerShip OtherActor)
    (:then
      (Class|PlayerShip|ProcessAsteroidCollision _asbp_player_ship))
    (:CastFailed
      (Utilities|Casting|CastToBP_Asteroid OtherActor
        (:then
          _)
        (:CastFailed
          (Utilities|Casting|CastToBP_Planet OtherActor)))))
  (Class|DestructibleComponent|ApplyDamage (Variables|Default|GetDestructibleAsteroid) 1.0 (Transformation|GetActorLocation) (Transformation|GetVelocity) 0.0)
  (Utilities|FlowControl|Delay 2.0)
  (Actor|DestroyActor))

(fn ConstructionScript
  (bind _asteroidmateriallist (Variables|Default|GetasteroidMaterialList))
  (bind _asteroidmateriallist_2 (Variables|Default|GetasteroidMaterialList))
  (bind _returnvalue (Utilities|Array|Length _asteroidmateriallist_2))
  (bind _returnvalue_2 (Math|Random|RandomInteger _returnvalue))
  (bind _output (Utilities|Array|Get(acopy) _asteroidmateriallist _returnvalue_2))
  (Rendering|Material|SetMaterial (Variables|Default|GetAsteroidSphere) 0 _output)
  (Rendering|Material|SetMaterial (Variables|Default|GetDestructibleAsteroid) 0 _output))